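; Saloon table configuration Blueprint that holds occupancy state for four seats.
; Every Tick it prints each seat's occupied flag to screen in red with zero duration, as a live debug readout.
; The graphs shown only read these flags, and the construction script is empty.
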(event `self.ReceiveTick`
  (params (DeltaSeconds :type "Float (single-precision)"))
  (`KismetSystemLibrary.PrintString` (`KismetStringLibrary.Conv_BoolToString` (`self.Seat1_Occupied`)) true true (struct :`R` 1.0 :`G` 0.020915 :`B` 0.000177 :`A` 1.0) 0.0)
  (`KismetSystemLibrary.PrintString` (`KismetStringLibrary.Conv_BoolToString` (`self.Seat2_Occupied`)) true true (struct :`R` 1.0 :`G` 0.020915 :`B` 0.000177 :`A` 1.0) 0.0)
  (`KismetSystemLibrary.PrintString` (`KismetStringLibrary.Conv_BoolToString` (`self.Seat3_Occupied`)) true true (struct :`R` 1.0 :`G` 0.020915 :`B` 0.000177 :`A` 1.0) 0.0)
  (`KismetSystemLibrary.PrintString` (`KismetStringLibrary.Conv_BoolToString` (`self.Seat4_Occupied`)) true true (struct :`R` 1.0 :`G` 0.020915 :`B` 0.000177 :`A` 1.0) 0.0))

(fn `UserConstructionScript`)