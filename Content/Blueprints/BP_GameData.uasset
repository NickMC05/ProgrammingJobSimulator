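; Game manager for a programming-office sim that runs a weekday-only clock, one game minute per second, and toggles NPC meeting priority.
; Saves and loads clock and programmer state on EndPlay and BeginPlay, matching NPCs by array order.
; When nobody has tasks, it assigns the player, then each NPC sequentially, LLM-written coding tasks via NVIDIA's API (hardcoded key), string-splitting responses into task structs.
; CreateNewTask targets the least-loaded programmer.
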(event `self.ReceiveBeginPlay`
  (`self.UpdateDateInSeconds`)
  (`self.LoadGameData`)
  (if (`self.DataLoadedStatus`) :!label _label
    (bind _totaltasks (`self.CountTotalCurrentTasks`))
    (if (== _totaltasks 0)
      (`self.GiveEveryoneTask`))
    (else
      (`KismetSystemLibrary.Delay` 0.1)
      (goto _label))))

(event `self.ReceiveTick`
  (params (DeltaSeconds :type "Float (single-precision)"))
  (`|ExecutionSequence`
    (:`then_0`
      (bind _returnvalue (`GameplayStatics.GetActorOfClass` "/Game/Blueprints/BP_FirstPersonCharacter.BP_FirstPersonCharacter_C")))
    (:`then_1`
      (bind _outactors (`GameplayStatics.GetAllActorsOfClass` "/Game/Characters/NPC_Base.NPC_Base_C"))
      (for _array_element _outactors
        _))))

(event `PostNVIDIA_Task`
  (params (Programmer :type "Actor Object Reference"))
  (bind _httpheader (make `HttpHeader`))
  (if true
    (bind _outrownames (`DataTableFunctionLibrary.GetDataTableRowNames` "/Game/DataTable/TaskNameList.TaskNameList"))
    (`HttpBlueprintFunctionLibrary.AddHeader` _httpheader "Accept" "application/json")
    (`HttpBlueprintFunctionLibrary.AddHeader` _httpheader "Content-Type" "application/json")
    (`HttpBlueprintFunctionLibrary.AddHeader` _httpheader "Authorization" "Bearer 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")
    (bind _returnvalue (`KismetStringLibrary.Conv_NameToString` (`|GetArrayItem` _outrownames (`KismetMathLibrary.RandomInteger` (`KismetArrayLibrary.Array_Length` _outrownames)))))
    (bind (_outheader _result_body) (`|HttpRequest` "https://integrate.api.nvidia.com/v1/chat/completions" "Post" _httpheader (`KismetStringLibrary.Concat_StrStr` "{ \n  \"model\": \"meta/llama-3.1-70b-instruct\", \n  \"temperature\": 0.2, \n  \"top_p\": 0.7, \n  \"frequency_penalty\": 0, \n  \"presence_penalty\": 0, \n  \"max_tokens\": 256, \n  \"stream\": false, \n  \"messages\": [ \n    {\"role\": \"user\", \"content\": \"" (`KismetStringLibrary.Concat_StrStr` "Play role as a CEO giving a coding algorithm assignment to one individual programmer. The assignment is about " _returnvalue ", which is doable by writing one file of code, can be cplusplus or python or etc. Do not give me the solution code. Deadline can be either 3-7 days depends on this task difficulty. Max 190 characters.") "\"} \n  ] \n}"))
      (:`then`
        (`KismetSystemLibrary.PrintString` "HTTP Processing")
        (set `self.LLM_ForTask_Running` false))
      (:`On Success`
        (`self.NVIDIA_Task_to_Struct` _result_body _returnvalue Programmer))
      (:`On Error`
        (`KismetSystemLibrary.PrintString` "HTTP Failed")
        (set `self.LLM_ForTask_Running` false)))))

(event `NVIDIA_Task_to_Struct`
  (params (NVIDIA_Output :type String) (TaskName :type String) (Programmer :type "Actor Object Reference"))
  (bind _lefts (`KismetStringLibrary.Split` (`.RightS` (`KismetStringLibrary.Split` NVIDIA_Output "\"content\":\"\\\"")) "\\\"\"},\"logprobs\":"))
  (bind _returnvalue (`KismetStringLibrary.Conv_StringToInt` (`KismetStringLibrary.Split` (`.RightS` (`KismetStringLibrary.Split` NVIDIA_Output "Deadline is ")) " days")))
  (if (> (`KismetStringLibrary.FindSubstring` NVIDIA_Output "\"content\":") -1)
    (bind _asbp_first_person_character (cast `/Game/Blueprints/BP_FirstPersonCharacter` Programmer)
      (:`then`
        (`KismetArrayLibrary.Array_Add` (`/Game/Blueprints/BP_FirstPersonCharacter.CurrentTasks` _asbp_first_person_character) (make `/Game/Structs/Task` TaskName _lefts _returnvalue))
        (set `self.LLM_ForTask_Running` false))
      (:`CastFailed`
        (bind _asnpc_base (cast `/Game/Characters/NPC_Base` Programmer))
        (`KismetArrayLibrary.Array_Add` (`/Game/Characters/NPC_Base.CurrentTasks` _asnpc_base) (make `/Game/Structs/Task` TaskName _lefts _returnvalue))
        (set `self.LLM_ForTask_Running` false)))
    (else
      (set `self.LLM_ForTask_Running` false))))

(event `UpdateDateInSeconds`
  (`|ExecutionSequence` :!label _label
    (:`then_0`
      (bind _output_get (set `self.Time_Minute` (+ (`self.Time_Minute`) 1)))
      (if (>= _output_get 60)
        (set `self.Time_Minute` 0)
        (bind _output_get_2 (set `self.Time_Hour` (+ (`self.Time_Hour`) 1)))
        (if (>= _output_get_2 24)
          (set `self.Time_Hour` 0)
          (switch `/Game/Enums/Day` (`self.Day`)
            (:`NewEnumerator0`
              (set `self.Day` "NewEnumerator1"))
            (:`NewEnumerator1`
              (set `self.Day` "NewEnumerator2"))
            (:`NewEnumerator2`
              (set `self.Day` "NewEnumerator3"))
            (:`NewEnumerator3`
              (set `self.Day` "NewEnumerator4"))
            (:`NewEnumerator4`
              (set `self.Day` "NewEnumerator0"))))))
    (:`then_1`
      (`KismetSystemLibrary.Delay` 1.0)
      (`KismetSystemLibrary.PrintString` (`KismetStringLibrary.Conv_IntToString` (`self.Time_Minute`)) true true (struct :`G` 0.66 :`B` 1.0 :`A` 1.0) 1.0)
      (`KismetSystemLibrary.PrintString` (`KismetStringLibrary.Conv_IntToString` (`self.Time_Hour`)) true true (struct :`G` 0.66 :`B` 1.0 :`A` 1.0) 1.0)
      (goto _label))))

(event `CreateNewTask`
  (bind _chosenprogrammer (`self.GetProgrammerWIthLowestTotalCurrentTasks`))
  (`self.PostNVIDIA_Task` _chosenprogrammer))

(event `GiveEveryoneTask`
  (bind _returnvalue (`GameplayStatics.GetActorOfClass` "/Game/Blueprints/BP_FirstPersonCharacter.BP_FirstPersonCharacter_C"))
  (`self.PostNVIDIA_Task` _returnvalue)
  (set `self.LLM_ForTask_Running` true)
  (if (`self.LLM_ForTask_Running`) :!label _label
    (`KismetSystemLibrary.Delay` 0.1)
    (goto _label)
    (else
      (bind _outactors (`GameplayStatics.GetAllActorsOfClass` "/Game/Characters/NPC_Base.NPC_Base_C"))
      (set `self.NPC_TemporaryIndexer` (- (`KismetArrayLibrary.Array_Length` _outactors) 1))
      (if (>= (`self.NPC_TemporaryIndexer`) 0) :!label _label_2
        (`self.PostNVIDIA_Task` (`|GetArrayItem` _outactors (`self.NPC_TemporaryIndexer`)))
        (set `self.LLM_ForTask_Running` true)
        (if (`self.LLM_ForTask_Running`) :!label _label_3
          (`KismetSystemLibrary.Delay` 0.1)
          (goto _label_3)
          (else
            (set `self.NPC_TemporaryIndexer` (- (`self.NPC_TemporaryIndexer`) 1))
            (goto _label_2)))))))

(event `LoadGameData`
  ; Load
  (bind _returnvalue (`GameplayStatics.DoesSaveGameExist` (`self.DataSaveSlot`)))
  (if _returnvalue
    (bind _returnvalue_2 (`GameplayStatics.LoadGameFromSlot` (`self.DataSaveSlot`)))
    (`|ExecutionSequence`
      (:`then_0`
        (bind _asbp_save_game (cast `/Game/Blueprints/BP_SaveGame` _returnvalue_2 :!pure true))
        (set `self.Time_Hour` (`/Game/Blueprints/BP_SaveGame.Time_Hour` _asbp_save_game))
        (set `self.Time_Minute` (`/Game/Blueprints/BP_SaveGame.Time_Minute` _asbp_save_game))
        (set `self.Day` (`/Game/Blueprints/BP_SaveGame.Day` _asbp_save_game)))
      (:`then_1`
        (bind _returnvalue_3 (`GameplayStatics.GetActorOfClass` "/Game/Blueprints/BP_FirstPersonCharacter.BP_FirstPersonCharacter_C"))
        (bind _output_currenttasks (break `/Game/Structs/CharacterData` (`|GetArrayItem` (`/Game/Blueprints/BP_SaveGame.Tasks` _asbp_save_game))))
        (set `/Game/Blueprints/BP_FirstPersonCharacter.CurrentTasks` _output_currenttasks _returnvalue_3)
        (bind _outactors (`GameplayStatics.GetAllActorsOfClass` "/Game/Characters/NPC_Base.NPC_Base_C"))
        (for (_array_element _array_index) _outactors
          (bind (_output_currenttasks_2 _output_energy _output_taskcompletion) (break `/Game/Structs/CharacterData` (`|GetArrayItem` (`/Game/Blueprints/BP_SaveGame.Tasks` _asbp_save_game) (+ _array_index 1))))
          (set `/Game/Characters/NPC_Base.CurrentTasks` _output_currenttasks_2 _array_element)
          (set `/Game/Characters/NPC_Base.Energy` _output_energy _array_element)
          (set `/Game/Characters/NPC_Base.TaskCompletion` _output_taskcompletion _array_element)))
      (:`then_2`
        (set `self.DataLoadedStatus` true)))
    (else
      (set `self.DataLoadedStatus` true))))

(event `self.ReceiveEndPlay`
  (params (EndPlayReason :type "EEndPlayReason Enum" :default "Destroyed"))
  ; Save
  (bind _returnvalue (`GameplayStatics.CreateSaveGameObject` "/Game/Blueprints/BP_SaveGame.BP_SaveGame_C"))
  (`|ExecutionSequence`
    (:`then_0`
      (set `/Game/Blueprints/BP_SaveGame.Time_Hour` (`self.Time_Hour`) _returnvalue)
      (set `/Game/Blueprints/BP_SaveGame.Time_Minute` (`self.Time_Minute`) _returnvalue)
      (set `/Game/Blueprints/BP_SaveGame.Day` (`self.Day`) _returnvalue))
    (:`then_1`
      (bind _returnvalue_2 (`GameplayStatics.GetActorOfClass` "/Game/Blueprints/BP_FirstPersonCharacter.BP_FirstPersonCharacter_C"))
      (`KismetArrayLibrary.Array_Add` (`/Game/Blueprints/BP_SaveGame.Tasks` _returnvalue) (make `/Game/Structs/CharacterData` (`/Game/Blueprints/BP_FirstPersonCharacter.CurrentTasks` _returnvalue_2)))
      (bind _outactors (`GameplayStatics.GetAllActorsOfClass` "/Game/Characters/NPC_Base.NPC_Base_C"))
      (for _array_element _outactors
        (`KismetArrayLibrary.Array_Add` (`/Game/Blueprints/BP_SaveGame.Tasks` _returnvalue) (make `/Game/Structs/CharacterData` (`/Game/Characters/NPC_Base.CurrentTasks` _array_element) (`/Game/Characters/NPC_Base.Energy` _array_element) (`/Game/Characters/NPC_Base.TaskCompletion` _array_element)))))
    (:`then_2`
      (`GameplayStatics.SaveGameToSlot` _returnvalue (`self.DataSaveSlot`)))))

(event `StartMeeting`
  (params (Individual :type "Actor Object Reference"))
  (if (not (`GameplayStatics.ObjectIsA` Individual "/Game/Characters/NPC_Base.NPC_Base_C"))
    (bind _outactors (`GameplayStatics.GetAllActorsOfClass` "/Game/Characters/NPC_Base.NPC_Base_C"))
    (for _array_element _outactors
      (set `/Game/Characters/NPC_Base.PriorityActivity` "NewEnumerator2" _array_element))))

(event `StopMeeting`
  (bind _outactors (`GameplayStatics.GetAllActorsOfClass` "/Game/Characters/NPC_Base.NPC_Base_C"))
  (for _array_element _outactors
    (if (`|EnumEquality` (`/Game/Characters/NPC_Base.PriorityActivity` _array_element) "NewEnumerator2")
      (set `/Game/Characters/NPC_Base.PriorityActivity` "NewEnumerator5" _array_element))))

(fn `CountTotalCurrentTasks`
  (returns (TotalTasks :type Integer))
  (locals (Count :type Integer))
  (set `local.Count` 0)
  (bind _outactors (`GameplayStatics.GetAllActorsOfClass` "/Game/Characters/NPC_Base.NPC_Base_C"))
  (for _array_element _outactors
    (set `local.Count` (+ (`KismetArrayLibrary.Array_Length` (`/Game/Characters/NPC_Base.CurrentTasks` _array_element)) (`local.Count`))))
  (bind _returnvalue (`GameplayStatics.GetActorOfClass` "/Game/Blueprints/BP_FirstPersonCharacter.BP_FirstPersonCharacter_C"))
  (return (+ (`KismetArrayLibrary.Array_Length` (`/Game/Blueprints/BP_FirstPersonCharacter.CurrentTasks` _returnvalue)) (`local.Count`))))

(fn `GetProgrammerWIthLowestTotalCurrentTasks`
  (returns (ChosenProgrammer :type "Actor Object Reference"))
  (locals (Programmer :type "Actor Object Reference") (CurrentTasksCount :type Integer))
  (bind _returnvalue (`GameplayStatics.GetActorOfClass` "/Game/Blueprints/BP_FirstPersonCharacter.BP_FirstPersonCharacter_C"))
  (set `local.Programmer` _returnvalue)
  (set `local.CurrentTasksCount` (`KismetArrayLibrary.Array_Length` (`/Game/Blueprints/BP_FirstPersonCharacter.CurrentTasks` _returnvalue)))
  (bind _outactors (`GameplayStatics.GetAllActorsOfClass` "/Game/Characters/NPC_Base.NPC_Base_C"))
  (for _array_element _outactors
    (bind _returnvalue_2 (`KismetArrayLibrary.Array_Length` (`/Game/Characters/NPC_Base.CurrentTasks` (cast `/Game/Characters/NPC_Base` _array_element :!pure true))))
    (if (< _returnvalue_2 (`local.CurrentTasksCount`))
      (set `local.Programmer` _array_element)
      (set `local.CurrentTasksCount` _returnvalue_2)))
  (return (`local.Programmer`)))

(fn `UserConstructionScript`)